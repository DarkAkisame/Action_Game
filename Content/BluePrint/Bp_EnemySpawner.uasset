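; Enemy spawner Blueprint that runs three sequential waves of enemies inside a box volume.
; A looping timer calls WaveCheck, which starts the next wave once the game mode reports no live enemies and the spawner is ready.
; Each wave has its own count and enemy class list, and SpawnWave places random picks at random points in the volume.
; Spawns adjust around collisions or are skipped, yet still count toward the wave total.
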(event Custom|WaveCheck
  ;[1 1 1] Wave check
  (if (and (== (Variables|/Game/BluePrint/BpGameMode.BpGameMode_C|GetLiveEnemies (Variables|Default|GetbpGameModeRef)) 0) (Variables|Default|GetbWaveReady))
    (switch int (Variables|Waves|GetWaveIndex)
      (:0
        (CallFunction|BeginWave)
        (CallFunction|SpawnWave (Utilities|Array|Get(acopy) (Variables|Default|GetWaveEnemieCount) (Variables|Waves|GetWaveIndex)) (Variables|Enemies|GetWavesEnemies1)))
      (:1
        (CallFunction|BeginWave)
        (CallFunction|SpawnWave (Utilities|Array|Get(acopy) (Variables|Default|GetWaveEnemieCount) (Variables|Waves|GetWaveIndex)) (Variables|Enemies|GetWavesEnemies2)))
      (:2
        (CallFunction|BeginWave)
        (CallFunction|SpawnWave (Utilities|Array|Get(acopy) (Variables|Default|GetWaveEnemieCount) (Variables|Waves|GetWaveIndex)) (Variables|Enemies|GetWavesEnemies3))))
    (Variables|Waves|SetWaveIndex (+ (Variables|Waves|GetWaveIndex) 1))))

(event EventBeginPlay
  ;[1 1 1] Event begin play spawnwave
  (bind _asbp_game_mode (Utilities|Casting|CastToBpGameMode (Game|GetGameMode)))
  (Variables|Default|SetbpGameModeRef _asbp_game_mode)
  (bind _returnvalue (Utilities|Time|SetTimerbyFunctionName 0 "WaveCheck" 1.0 true))
  (Variables|Default|SetWaveTimer _returnvalue))

(fn ConstructionScript)

(fn BeginWave
  (Variables|Default|SetbWaveReady false)
  (Variables|Waves|SetWaveActive 0))

(fn SpawnWave
  (params (WaveTotal :type Integer) (WaveEnemies :type Array%20of%20Bp%20Enemy%20Class%20References))
  (bind _spawnvalume (Variables|Default|GetSpawnValume))
  (for _index (range 0 (+ WaveTotal 1))
    (if (> WaveTotal (Variables|Waves|GetWaveActive))
      (if (not (Variables|Default|GetbWaveReady))
        (Game|SpawnActorfromClass (Utilities|Array|Get(acopy) WaveEnemies (Math|Random|RandomInteger (Utilities|Array|Length WaveEnemies))) (Math|Conversions|ToTransform(Vector) (Math|Random|RandomPointinBoundingBox (Transformation|GetWorldLocation _spawnvalume) (Components|Box|GetScaledBoxExtent _spawnvalume))) "AdjustIfPossibleButDontSpawnIfColliding" 0 0)
        (Variables|Waves|SetWaveActive (+ (Variables|Waves|GetWaveActive) 1)))
      (else
        (Variables|Default|SetbWaveReady true)))))