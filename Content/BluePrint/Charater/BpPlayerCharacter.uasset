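; Player character Blueprint that mirrors health, mana and strength changes onto the player's HUD.
; Each change event casts the controller to BpPlayerControllerBase and sets the matching glass ball widget on MainHUD to the current-to-maximum ratio.
; Updates are purely event-driven and are skipped when the controller cast fails.
; BeginPlay and the construction script only call their parents, and Tick is disabled.
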(event EventBeginPlay
  (|CallParentFunction))

(event Collision|EventActorBeginOverlap
  (params (OtherActor :type Actor%20Object%20Reference))
  (|CallParentFunction OtherActor) ; This node is disabled and will not be called.\nDrag off pins to build functionality.
)

(event EventTick
  (params (DeltaSeconds :type Float%20%28single-precision%29))
  (|CallParentFunction DeltaSeconds) ; This node is disabled and will not be called.\nDrag off pins to build functionality.
)

(event EventOnHealthChanged
  (params (Health :type Float%20%28single-precision%29) (MaxHealth :type Float%20%28single-precision%29))
  (bind _asbp_player_controller_base (Utilities|Casting|CastToBpPlayerControllerBase (Pawn|GetController)))
  (Default|SetPercentage (Variables|/Game/UI/Bpw_HuD_Main.Bpw_HuD_Main_C|GetHealth_GlassBall (Variables|/Game/BluePrint/BpPlayerControllerBase.BpPlayerControllerBase_C|GetMain_HUD _asbp_player_controller_base)) (/ Health MaxHealth)))

(event EventOnManaChanged
  (params (Mana :type Float%20%28single-precision%29) (MaxMana :type Float%20%28single-precision%29))
  (bind _asbp_player_controller_base (Utilities|Casting|CastToBpPlayerControllerBase (Pawn|GetController)))
  (Default|SetPercentage (Variables|/Game/UI/Bpw_HuD_Main.Bpw_HuD_Main_C|GetManaGlassBall (Variables|/Game/BluePrint/BpPlayerControllerBase.BpPlayerControllerBase_C|GetMain_HUD _asbp_player_controller_base)) (/ Mana MaxMana)))

(event EventOnStrengthChanged
  (params (Strength :type Float%20%28single-precision%29) (MaxStrengtha :type Float%20%28single-precision%29))
  (bind _asbp_player_controller_base (Utilities|Casting|CastToBpPlayerControllerBase (Pawn|GetController)))
  (Default|SetPercentage (Variables|/Game/UI/Bpw_HuD_Main.Bpw_HuD_Main_C|GetStrengthGlassBall (Variables|/Game/BluePrint/BpPlayerControllerBase.BpPlayerControllerBase_C|GetMain_HUD _asbp_player_controller_base)) (/ Strength MaxStrengtha)))

(fn ConstructionScript
  (|CallParentFunction))