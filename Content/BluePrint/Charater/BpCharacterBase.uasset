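; Base character Blueprint for Gameplay Ability System combat, covering melee combos, dash hits, pushback with stun, and death.
; BeginPlay grants initial abilities and regen; melee input activates the melee ability, or confirms the target while targeting.
; Sword and capsule overlaps send damage gameplay events to itself for hostile characters, with dash hits deduplicated by an exclusion array.
; DetermingCombo cycles three montages and damage levels; pushback resets the combo and briefly zeroes ground friction.
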(event OnComponentBeginOverlap(SwordColider)
  (params (OverlappedComponent :type Primitive%20Component%20Object%20Reference) (OtherActor :type Actor%20Object%20Reference) (OtherComp :type Primitive%20Component%20Object%20Reference) (OtherBodyIndex :type Integer) (bFromSweep :type Boolean) (SweepResult :type Hit%20Result%20Structure%20%28by%20ref%29))
  ;[1 1 1] Sword collider
  (if (!= OtherActor self)
    (bind _asbp_character_base (Utilities|Casting|CastToBpCharacterBase OtherActor))
    (bind _returnvalue (Class|CharacterBase|IsOtherHostile _asbp_character_base self))
    (if _returnvalue
      (Ability|SendGameplayEventtoActor self "(TagName=\"Skill.Melee.DealDamage\")" (Utilities|Struct|MakeGameplayEventData "" 0 OtherActor)))))

(event OnComponentBeginOverlap(CapsuleComponent)
  (params (OverlappedComponent :type Primitive%20Component%20Object%20Reference) (OtherActor :type Actor%20Object%20Reference) (OtherComp :type Primitive%20Component%20Object%20Reference) (OtherBodyIndex :type Integer) (bFromSweep :type Boolean) (SweepResult :type Hit%20Result%20Structure%20%28by%20ref%29))
  (bind _self self)
  (bind _overlapactorexlude (Variables|Default|GetOverLapActorExlude))
  ;[1 1 1] Dash/arrayof hit and call to damage
  (bind _asbp_character_base (Utilities|Casting|CastToBpCharacterBase OtherActor))
  (bind _returnvalue (Class|CharacterBase|IsOtherHostile _asbp_character_base _self))
  (if _returnvalue
    (if (not (Utilities|Array|ContainsItem _overlapactorexlude _asbp_character_base))
      (Utilities|Array|AddUnique _overlapactorexlude _asbp_character_base)
      (Ability|SendGameplayEventtoActor _self "(TagName=\"Skill.Dash.Damage\")" (Utilities|Struct|MakeGameplayEventData "" _self OtherActor)))))

(event Custom|MeleeAttack
  (bind _abilitysystemcomp (Variables|Default|GetAbilitySystemComp))
  ;[1 1 1] Melee set up
  (if (Variables|Default|GetTargetting)
    (Class|AbilitySystemComponent|TargetConfirm _abilitysystemcomp)
    (else
      (Abilities|TryActivateAbilitybyClass _abilitysystemcomp "/Game/BluePrint/Charater/GameplayAbilitys/Melee/Ga_Melee.Ga_Melee_C" true))))

(event Custom|MakeCamerControlRotation
  (params (ShouldControlRotation :type Boolean))
  (if ShouldControlRotation
    (Variables|Default|SetbUseControllerRotationYaw true)
    (Variables|/Script/Engine.CharacterMovementComponent|SetbOrientRotationToMovement (Variables|Character|GetCharacterMovement) false)
    (else
      (Variables|Default|SetbUseControllerRotationYaw false)
      (Variables|/Script/Engine.CharacterMovementComponent|SetbOrientRotationToMovement (Variables|Character|GetCharacterMovement) true))))

(event Custom|EndCombo
  ;[1 1 1] Melee set up
  (Variables|Default|SetComboCount 1))

(event Custom|PushingCharacter
  (params (ImpulseDirection :type Vector) (PushStrangth :type Float%20%28single-precision%29) (StunDuration :type Float%20%28single-precision%29) (PushAnim :type Anim%20Montage%20Object%20Reference))
  (bind _charactermovement (Variables|Character|GetCharacterMovement))
  ;[1 1 1] PUSH BACK // Stun
  (CallFunction|EndCombo)
  (Animation|PlayAnimMontage PushAnim 1.0 "None")
  (Variables|Default|SetDefaultGroundFriction (Variables|/Script/Engine.CharacterMovementComponent|GetGroundFriction _charactermovement))
  (Variables|/Script/Engine.CharacterMovementComponent|SetGroundFriction _charactermovement 0.0)
  (Physics|AddImpulse _charactermovement (* ImpulseDirection PushStrangth) true)
  (if (> StunDuration 0.0)
    (Class|CharacterBase|HitStun StunDuration))
  (Utilities|FlowControl|Delay 0.3)
  (Variables|/Script/Engine.CharacterMovementComponent|SetGroundFriction _charactermovement (Variables|Default|GetDefaultGroundFriction)))

(event EventBeginPlay
  (Class|CharacterBase|AquireAbilies (Variables|Default|GetInitialAbilities))
  (GameplayEffects|ApplyGameplayEffectToSelf :self (Variables|Default|GetAbilitySystemComp) :GameplayEffectClass "/Game/BluePrint/Charater/GameplayAbilitys/GeneralGameplayEfect/Ge_BasicRegen.Ge_BasicRegen_C"))

(event EventDie
  ;[1 1 1] Death
  (bind _returnvalue (Animation|PlayAnimMontage "/Game/BluePrint/Charater/Animation/Am_ShinbiDeath.Am_ShinbiDeath" 1.0 "None"))
  (Utilities|FlowControl|Delay _returnvalue)
  (Actor|DestroyActor))

(fn ConstructionScript)

(fn SetCollisontoPaw
  (params (NewCollisonResponse :type ECollisionResponse%20Enum :default "ECR_Ignore"))
  (Collision|SetCollisionResponsetoChannel (Variables|Default|GetCapsuleComponent) "ECC_Pawn" NewCollisonResponse))

(fn DetermingCombo
  (switch int (Variables|Default|GetComboCount)
    (:1
      (Variables|Default|SetMeleeMontage "/Game/BluePrint/Charater/Animation/AmShinbiMelee_Combo_01.AmShinbiMelee_Combo_01")
      (Math|Integer|IncrementInt (Variables|Default|GetComboCount)
        (:%20%20
          (Variables|Default|SetMC_DamageLevel 1))))
    (:2
      (Variables|Default|SetMeleeMontage "/Game/BluePrint/Charater/Animation/AmShinbiMelee_Combo_02.AmShinbiMelee_Combo_02")
      (Math|Integer|IncrementInt (Variables|Default|GetComboCount)
        (:%20%20
          (Variables|Default|SetMC_DamageLevel 2))))
    (:3
      (Variables|Default|SetMeleeMontage "/Game/BluePrint/Charater/Animation/AmShinbiMelee_Combo_03.AmShinbiMelee_Combo_03")
      (Variables|Default|SetComboCount 1)
      (Variables|Default|SetMC_DamageLevel 3))))