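; Fire Blast gameplay ability that pulls surrounding characters toward the caster, then damages and blasts them away.
; It commits, starts the UI cooldown and plays a montage, ending when the montage finishes.
; A Pull gameplay event triggers instant radius targeting, caching the targets and pulling them with a stun.
; A later Push event applies damage and stunning knockback to those targets, taking every push direction from the last pulled character.
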(event Ability|EventActivateAbility
  (Ability|CommitAbility)
  (CallFunction|DoUICoolDown)
  (|PlayMontageandWaitProxy "None" "/Game/BluePrint/Charater/Animation/Am_Shinbo_FireBLast.Am_Shinbo_FireBLast" 1.0 "None" true 1.0
    (:then
      (Ability|Tasks|WaitGameplayEvent "(TagName=\"Skill.FireBlast.Pull\")" 0
        (:EventReceived
          (bind _data (|WaitTargetData :ConfirmationType "Instant" :Class "/Script/ActionGame.Ga_TargetActor_Around" :Radius 6e+02 :ReticleClass 0)
            (:then
              (Ability|Tasks|WaitGameplayEvent "(TagName=\"Skill.FireBlast.Push\")" 0
                (:EventReceived
                  (GameplayEffects|ApplyGameplayEffectToTarget (Variables|Default|GetTargetDataHandel) "/Game/BluePrint/Charater/GameplayAbilitys/FIreBlast/Ge_FireBLastDamge.Ge_FireBLastDamge_C" 1 1)
                  (for _array_element (Ability|TargetData|GetActorsfromTargetData (Variables|Default|GetTargetDataHandel))
                    (bind _asbp_character_base (Utilities|Casting|CastToBpCharacterBase _array_element))
                    (Default|PushingCharacter _asbp_character_base (* (Math|Vector|Normalize (- (Transformation|GetActorLocation (Ability|GetOwningActorfromActorInfo)) (Transformation|GetActorLocation (stale _asbp_character_base_2)))) -1.0) 2e+03 2.0)))))
            (:ValidData
              (Variables|Default|SetTargetDataHandel _data)
              (for _array_element_2 (Ability|TargetData|GetActorsfromTargetData _data)
                (bind _asbp_character_base_2 (Utilities|Casting|CastToBpCharacterBase _array_element_2))
                (Default|PushingCharacter _asbp_character_base_2 (Math|Vector|Normalize (- (Transformation|GetActorLocation (Ability|GetOwningActorfromActorInfo)) (Transformation|GetActorLocation _asbp_character_base_2))) 1e+03 3.0 "/Game/BluePrint/Charater/Animation/Am_HIt_attack.Am_HIt_attack")))))))
    (:OnCompleted
      (Ability|EndAbility :!label _label))
    (:OnBlendOut
      (goto _label))
    (:OnInterrupted
      (goto _label))
    (:OnCancelled
      (goto _label))))

(event Ability|EventOnEndAbility
  (params (bWasCancelled :type Boolean)))