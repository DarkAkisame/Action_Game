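; Laser beam actor that signals damage to its instigator for hostile characters caught at the beam's end.
; LazerEnd overlaps maintain a list of hostile characters, which a looping timer sends as target data in a Skill.Lazer.DealDamage gameplay event.
; Each tick, it stretches the mesh to LazerEnd by setting an end-bone offset in the anim Blueprint from the change in original length.
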(event OnComponentBeginOverlap(LazerEnd)
  (params (OverlappedComponent :type Primitive%20Component%20Object%20Reference) (OtherActor :type Actor%20Object%20Reference) (OtherComp :type Primitive%20Component%20Object%20Reference) (OtherBodyIndex :type Integer) (bFromSweep :type Boolean) (SweepResult :type Hit%20Result%20Structure%20%28by%20ref%29))
  (bind _asbp_character_base (Utilities|Casting|CastToBpCharacterBase OtherActor))
  (bind _asbp_character_base_2 (Utilities|Casting|CastToBpCharacterBase (Game|GetInstigator)))
  (bind _returnvalue (Class|CharacterBase|IsOtherHostile _asbp_character_base_2 _asbp_character_base))
  (if _returnvalue
    (Utilities|Array|AddUnique (Variables|Default|GetOverLapingActors) _asbp_character_base)))

(event OnComponentEndOverlap(LazerEnd)
  (params (OverlappedComponent :type Primitive%20Component%20Object%20Reference) (OtherActor :type Actor%20Object%20Reference) (OtherComp :type Primitive%20Component%20Object%20Reference) (OtherBodyIndex :type Integer))
  (bind _asbp_character_base (Utilities|Casting|CastToBpCharacterBase OtherActor))
  (Utilities|Array|RemoveItem (Variables|Default|GetOverLapingActors) _asbp_character_base))

(event Custom|SendDealDamageEvent
  (bind _overlapingactors (Variables|Default|GetOverLapingActors))
  ;[1 1 1] SendDamagePer .3sec
  (if (Math|Conversions|ToBoolean(Integer) (Utilities|Array|Length _overlapingactors))
    (Ability|SendGameplayEventtoActor (Game|GetInstigator) "(TagName=\"Skill.Lazer.DealDamage\")" (Utilities|Struct|MakeGameplayEventData "" 0 0 0 0 "()" "(GameplayTags=)" "(GameplayTags=)" 0.0 (Ability|TargetData|AbilityTargetDatafromActorArray _overlapingactors)))))

(event EventBeginPlay
  (Variables|Default|SetLazerOriginalLangth (Math|Vector|VectorLength (- (Transformation|GetSocketLocation (Variables|Default|GetLazerMesh) "end") (Transformation|GetActorLocation))))
  ;[1 1 1] SendDamagePer .3sec
  (Utilities|Time|SetTimerbyEvent (delegate Custom|SendDealDamageEvent) 0.3 true))

(event Collision|EventActorBeginOverlap
  (params (OtherActor :type Actor%20Object%20Reference)))

(event EventTick
  (params (DeltaSeconds :type Float%20%28single-precision%29))
  (bind _asanim_bp_lazer (Utilities|Casting|CastToAnim_Bp_Lazer (Components|SkeletalMesh|GetAnimInstance (Variables|Default|GetLazerMesh))))
  (Variables|/Game/BluePrint/Charater/GameplayAbilitys/Lazer/LazerAssets/Anim_Bp_Lazer.Anim_Bp_Lazer_C|SetEndBoneOffSet _asanim_bp_lazer (Math|Vector|MakeVector (- (Math|Vector|VectorLength (- (Transformation|GetWorldLocation (Variables|Default|GetLazerEnd)) (Transformation|GetActorLocation))) (Variables|Default|GetLazerOriginalLangth)) 0.0 0.0)))

(fn ConstructionScript)