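; Gameplay ability for a channeled laser skill that damages and knocks back targets while its cost stays affordable.
; On activation it commits, starts the UI cooldown, plays a montage, then attaches a Bp_Lazer actor to the mesh and enables camera-controlled rotation.
; Damage gameplay events apply the damage effect and push targets away from the beam end, or end the ability if cost is unavailable.
; Ending removes the mana-cost effect, restores rotation and destroys the laser.
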(event Ability|EventActivateAbility
  (Ability|CommitAbility)
  (CallFunction|DoUICoolDown)
  (|PlayMontageandWaitProxy "None" "/Game/BluePrint/Charater/Animation/Am_Shinbi_Lazer.Am_Shinbi_Lazer" 1.0 "None" true 1.0
    (:then
      (Utilities|FlowControl|Delay 0.2)
      (bind _basecharacterref (CallFunction|GetPlayerInfoRef))
      (bind _spawnedactor (|SpawnActor :Class "/Game/BluePrint/Charater/GameplayAbilitys/Lazer/Bp_Lazer.Bp_Lazer_C" :Instigator _basecharacterref)
        (:then
          (bind _output_get (Variables|Default|SetLazerActor _spawnedactor))
          (Transformation|AttachComponentToComponent _output_get (Variables|/Script/Engine.Character|GetMesh _basecharacterref) "Lazer" "SnapToTarget" "SnapToTarget" "SnapToTarget" true)
          (Default|MakeCamerControlRotation _basecharacterref true)
          (bind _payload (Ability|Tasks|WaitGameplayEvent "(TagName=\"Skill.Lazer.DealDamage\")" 0)
            (:EventReceived
              (bind _cancast (CallFunction|IsCostStillAvaliable))
              (if _cancast
                (GameplayEffects|ApplyGameplayEffectToTarget (.TargetData (Utilities|Struct|BreakGameplayEventData _payload)) "/Game/BluePrint/Charater/GameplayAbilitys/Lazer/Ge_LazerDamage.Ge_LazerDamage_C" 1 1)
                (for _array_element (Ability|TargetData|GetActorsfromTargetData (.TargetData (Utilities|Struct|BreakGameplayEventData _payload)))
                  (bind _asbp_character_base (Utilities|Casting|CastToBpCharacterBase _array_element))
                  (Default|PushingCharacter _asbp_character_base (Math|Vector|Normalize (- (Transformation|GetActorLocation _asbp_character_base) (Transformation|GetWorldLocation (Variables|/Game/BluePrint/Charater/GameplayAbilitys/Lazer/Bp_Lazer.Bp_Lazer_C|GetLazerEnd (.AsBp%20Lazer (Utilities|Casting|CastToBp_Lazer (Variables|Default|GetLazerActor))))))) 5e+02 0.3 "/Game/BluePrint/Charater/Animation/Am_HIt_attack.Am_HIt_attack"))
                (else
                  (Ability|EndAbility))))))))))

(event Ability|EventOnEndAbility
  (params (bWasCancelled :type Boolean))
  (Ability|RemoveGameplayEffectFromOwnerWithAssetTags "(GameplayTags=((TagName=\"Skill.Lazer.ManaCost\")))")
  (bind _basecharacterref (CallFunction|GetPlayerInfoRef))
  (Default|MakeCamerControlRotation _basecharacterref false)
  (Actor|DestroyActor (Variables|Default|GetLazerActor)))