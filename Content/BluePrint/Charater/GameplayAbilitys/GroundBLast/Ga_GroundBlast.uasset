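; Gameplay Ability for Ground Blast, a ground-targeted area attack that damages characters and knocks them upward with a stun.
; If the cost is affordable, it plays a targeting montage, waits out its length, then awaits user-confirmed data from a ground-select target actor.
; Confirmation commits the ability, starts the UI cooldown and plays the cast montage, spawning the blast particle and applying damage and push to targets.
; The Targetting flag on the character clears on confirmation and when the ability ends.
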(event Ability|EventActivateAbility
  (bind _cancast (CallFunction|IsCostStillAvaliable))
  (if _cancast
    (|PlayMontageandWaitProxy "None" "/Game/BluePrint/Charater/Animation/Am_SinbiTargetting.Am_SinbiTargetting" 1.0 "StartNone" true 1.0
      (:then
        (Utilities|FlowControl|Delay (Variables|/Script/Engine.AnimSequenceBase|GetSequenceLength (Animation|GetCurrentMontage :!class /Script/GameplayAbilities.GameplayAbility)))
        (bind _data (|WaitTargetData :ConfirmationType "UserConfirmed" :Class "/Game/BluePrint/Charater/GameplayAbilitys/GroundBLast/Bp_GA_TargetActorSelectGround.Bp_GA_TargetActorSelectGround_C" :ReticleClass 0)
          (:ValidData
            (bind _basecharacterref (CallFunction|GetPlayerInfoRef))
            (Variables|/Game/BluePrint/Charater/BpCharacterBase.BpCharacterBase_C|SetTargetting _basecharacterref false)
            (Ability|CommitAbility)
            (CallFunction|DoUICoolDown)
            (|PlayMontageandWaitProxy "None" "/Game/BluePrint/Charater/Animation/Am_GroundBlast_Cast.Am_GroundBlast_Cast" 1.0 "None" true 1.0
              (:then
                (Effects|SpawnEmitteratLocation "/Game/BluePrint/Charater/GameplayAbilitys/GroundBLast/P_groundBlast.P_groundBlast" (Class|AbilitySystemBlueprintLibrary|GetTargetDataEndPoint _data (- (Ability|TargetData|GetDataCountfromTargetData _data) 1)))
                (GameplayEffects|ApplyGameplayEffectToTarget _data "/Game/BluePrint/Charater/GameplayAbilitys/GroundBLast/Ge_GroundBlast_Damage.Ge_GroundBlast_Damage_C" 1 1)
                (for _array_element (Ability|TargetData|GetActorsfromTargetData _data)
                  (bind _asbp_character_base (Utilities|Casting|CastToBpCharacterBase _array_element))
                  (Default|PushingCharacter _asbp_character_base "0, 0,1.000000" 5e+02 2.0)))
              (:OnCompleted
                (Ability|EndAbility :!label _label))
              (:OnBlendOut
                (goto _label))
              (:OnInterrupted
                (goto _label))
              (:OnCancelled
                (goto _label))))
          (:Cancelled
            (Ability|EndAbility)))))
    (else
      (Ability|EndAbility))))

(event Ability|EventOnEndAbility
  (params (bWasCancelled :type Boolean))
  (bind _basecharacterref (CallFunction|GetPlayerInfoRef))
  (Variables|/Game/BluePrint/Charater/BpCharacterBase.BpCharacterBase_C|SetTargetting _basecharacterref false))