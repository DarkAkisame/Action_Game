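; Base Gameplay Ability Blueprint that provides shared player lookup and HUD cooldown helpers.
; GetPlayerInfoRef casts the owning actor to the base character, then its controller to the base player controller.
; DoUICoolDown uses that controller to scan the main HUD's slots and starts the cooldown on any whose ability class matches this ability's info.
; Activate and end events are unimplemented here.
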(event Ability|EventActivateAbility)

(event Ability|EventOnEndAbility
  (params (bWasCancelled :type Boolean)))

(fn GetPlayerInfoRef
  (bind _asbp_character_base (Utilities|Casting|CastToBpCharacterBase (Ability|GetOwningActorfromActorInfo))
    (:then
      (bind _asbp_player_controller_base (Utilities|Casting|CastToBpPlayerControllerBase (Pawn|GetController _asbp_character_base))
        (:then
          _)
        (:CastFailed
          _)))
    (:CastFailed
      _))
  (return _asbp_character_base _asbp_player_controller_base))

(fn DoUICoolDown
  (bind _basecontrollerref (CallFunction|GetPlayerInfoRef))
  (Utilities|IsValid _basecontrollerref
    (:Is%20Valid
      (for _array_element (Variables|/Game/UI/Bpw_HuD_Main.Bpw_HuD_Main_C|GetSlots (Variables|/Game/BluePrint/BpPlayerControllerBase.BpPlayerControllerBase_C|GetMain_HUD _basecontrollerref))
        (bind _returnvalue (Class|GameplayAbilityBase|GetAbilityInfo))
        (if (== (.abilityclass (Variables|/Game/UI/Bpw_AbilitySlot.Bpw_AbilitySlot_C|GetAbilityInfo _array_element)) (.abilityclass _returnvalue))
          (Default|StartCooldown _array_element))))))