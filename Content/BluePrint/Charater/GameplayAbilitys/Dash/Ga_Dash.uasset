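; Dash gameplay ability that launches the owning character forward, damaging and knocking back characters it hits.
; On activation it commits, starts the UI cooldown, zeroes ground friction, applies a forward velocity impulse and sets pawn collision to overlap.
; While the dash montage plays, Skill.Dash.Damage events apply a damage effect and push the target away with a stun and hit animation.
; Any montage ending restores friction and blocking collision, then ends the ability.
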(event Ability|EventActivateAbility
  (Ability|CommitAbility)
  (CallFunction|DoUICoolDown)
  (bind _ascharacter (Utilities|Casting|CastToCharacter (Ability|GetOwningActorfromActorInfo))
    (:then
      (Variables|Default|SetOrigenalGroundFiction (Variables|/Script/Engine.CharacterMovementComponent|GetGroundFriction (Variables|/Script/Engine.Character|GetCharacterMovement _ascharacter)))
      (Variables|/Script/Engine.CharacterMovementComponent|SetGroundFriction (Variables|/Script/Engine.Character|GetCharacterMovement _ascharacter) 0.0)
      (Physics|AddImpulse (Variables|/Script/Engine.Character|GetCharacterMovement _ascharacter) (* (Transformation|GetActorForwardVector _ascharacter) 2e+03) true)
      (bind _basecharacterref (CallFunction|GetPlayerInfoRef))
      (Default|SetCollisontoPaw _basecharacterref "ECR_Overlap")
      (|PlayMontageandWaitProxy "None" "/Game/BluePrint/Charater/Animation/Am_ShinbiDash.Am_ShinbiDash" 1.0 "None" true 1.0
        (:then
          (bind _payload (Ability|Tasks|WaitGameplayEvent "(TagName=\"Skill.Dash.Damage\")" 0)
            (:EventReceived
              (GameplayEffects|ApplyGameplayEffectToTarget (Ability|TargetData|AbilityTargetDatafromActor (.Target (Utilities|Struct|BreakGameplayEventData _payload))) "/Game/BluePrint/Charater/GameplayAbilitys/Dash/Ge_DashDamage.Ge_DashDamage_C" 1 1)
              (bind _asbp_character_base (Utilities|Casting|CastToBpCharacterBase (.Target (Utilities|Struct|BreakGameplayEventData _payload))))
              (Default|PushingCharacter _asbp_character_base (Math|Vector|Normalize (- (Transformation|GetActorLocation _asbp_character_base) (Transformation|GetActorLocation (Ability|GetOwningActorfromActorInfo)))) 4e+03 1.6 "/Game/BluePrint/Charater/Animation/Am_HIt_attack.Am_HIt_attack"))))
        (:OnCompleted
          (Variables|/Script/Engine.CharacterMovementComponent|SetGroundFriction (Variables|/Script/Engine.Character|GetCharacterMovement _ascharacter) (Variables|Default|GetOrigenalGroundFiction) :!label _label)
          (Default|SetCollisontoPaw _basecharacterref "ECR_Block")
          (Ability|EndAbility :!label _label_2))
        (:OnBlendOut
          (goto _label))
        (:OnInterrupted
          (goto _label))
        (:OnCancelled
          (goto _label))))
    (:CastFailed
      (goto _label_2))))

(event Ability|EventOnEndAbility
  (params (bWasCancelled :type Boolean)))