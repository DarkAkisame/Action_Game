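; Base player controller that creates the main HUD, forwards new abilities to its slots, and routes player input to the controlled character.
; Axis inputs drive look and movement through a camera-vector helper, while actions trigger jump, melee attack and target cancel.
; Five slot inputs share TryActivateAbilitySlot, which reads the class from the HUD, activates it through GAS, flags targeting abilities, calls TargetCancel and ends the combo.
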(event EventBeginPlay
  (bind _returnvalue (UserInterface|CreateWidget "/Game/UI/Bpw_HuD_Main.Bpw_HuD_Main_C"))
  (Variables|Default|SetMain_HUD _returnvalue)
  (UserInterface|Viewport|AddtoViewport _returnvalue 0))

(event EventTick
  (params (DeltaSeconds :type Float%20%28single-precision%29)))

(event EventAddAbilitytoUI
  (params (AbilityInfo :type Gameplay%20Ability%20Info%20Structure))
  (Default|AddAbilitytoSlots (Variables|Default|GetMain_HUD) AbilityInfo))

(event Input|ActionEvents|InputActionJump
  (params (Key :type Key%20Structure))
  ;[1 1 1] Basic Movement
  (:Pressed
    (bind _asbp_character_base (Utilities|Casting|CastToBpCharacterBase (Pawn|GetControlledPawn)))
    (Character|Jump _asbp_character_base)))

(event Input|ActionEvents|InputActionPrimaryAttack
  (params (Key :type Key%20Structure))
  (:Pressed
    (bind _asbp_character_base (Utilities|Casting|CastToBpCharacterBase (Pawn|GetControlledPawn)))
    (Default|MeleeAttack _asbp_character_base)))

(event Input|ActionEvents|InputActionCancel
  (params (Key :type Key%20Structure))
  (:Pressed
    (bind _asbp_character_base (Utilities|Casting|CastToBpCharacterBase (Pawn|GetControlledPawn)))
    (Class|AbilitySystemComponent|TargetCancel (Ability|GetAbilitySystemComponent _asbp_character_base))))

(event Input|ActionEvents|InputActionSlotOneAbility
  (params (Key :type Key%20Structure))
  (:Pressed
    (CallFunction|TryActivateAbilitySlot)))

(event Input|ActionEvents|InputActionSlotTwoAbility
  (params (Key :type Key%20Structure))
  (:Pressed
    (CallFunction|TryActivateAbilitySlot 1)))

(event Input|ActionEvents|InputActionSlortThreeAbility
  (params (Key :type Key%20Structure))
  (:Pressed
    (CallFunction|TryActivateAbilitySlot 2)))

(event Input|ActionEvents|InputActionSlotFourAbility
  (params (Key :type Key%20Structure))
  (:Pressed
    (CallFunction|TryActivateAbilitySlot 3)))

(event Input|ActionEvents|InputActionSlotFiveAbility
  (params (Key :type Key%20Structure))
  (:Pressed
    (CallFunction|TryActivateAbilitySlot 4)))

(event Input|AxisEvents|InputAxisMoveForward
  (params (AxisValue :type Float%20%28single-precision%29))
  ;[1 1 1] Basic Movement
  (Pawn|Input|AddMovementInput (Pawn|GetControlledPawn) (.CamerasForward (Utilities|GetCameraForwardVector)) AxisValue false))

(event Input|AxisEvents|InputAxisMoveRight
  (params (AxisValue :type Float%20%28single-precision%29))
  ;[1 1 1] Basic Movement
  (Pawn|Input|AddMovementInput (Pawn|GetControlledPawn) (.CamerasRight (Utilities|GetCameraForwardVector)) AxisValue false))

(event Input|AxisEvents|InputAxisLookingUp
  (params (AxisValue :type Float%20%28single-precision%29))
  ;[1 1 1] Basic Movement
  (Class|PlayerController|AddPitchInput AxisValue))

(event Input|AxisEvents|InputAxisLookingRight
  (params (AxisValue :type Float%20%28single-precision%29))
  ;[1 1 1] Basic Movement
  (Class|PlayerController|AddYawInput AxisValue))

(fn ConstructionScript)

(fn TryActivateAbilitySlot
  (params (SlotNumber :type Integer))
  (bind (_abilityclass _valid) (Default|GetSlotAbilityClass (Variables|Default|GetMain_HUD) SlotNumber))
  (if _valid
    (bind _asbp_character_base (Utilities|Casting|CastToBpCharacterBase (Pawn|GetControlledPawn)))
    (Abilities|TryActivateAbilitybyClass (Ability|GetAbilitySystemComponent _asbp_character_base) _abilityclass true)
    (Utilities|Casting|CastToBp_Gameplay_Ability_TargettypeClass _abilityclass
      (:then
        (Variables|/Game/BluePrint/Charater/BpCharacterBase.BpCharacterBase_C|SetTargetting _asbp_character_base true))
      (:CastFailed
        (Variables|/Game/BluePrint/Charater/BpCharacterBase.BpCharacterBase_C|SetTargetting _asbp_character_base false)))
    (Class|AbilitySystemComponent|TargetCancel (Ability|GetAbilitySystemComponent _asbp_character_base))
    (Default|EndCombo _asbp_character_base)))