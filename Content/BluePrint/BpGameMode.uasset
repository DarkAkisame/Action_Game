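; Game mode Blueprint that spawns enemy bots at locations chosen by the Environment Query System.
; SpawnNewBot runs Eqs_FindSpawnLocation in random-best-25% mode and binds a handler for query completion.
; On success, the handler draws a debug sphere at each result and spawns BpEnemy there, adjusting for collisions or skipping blocked spots.
; A disconnected timer setup for Bp_EnemySpawner remains in the graph but never runs.
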(event Custom|SpawnQueryFinishedEvent
  (params (QueryInstance :type Env%20Query%20Instance%20Blueprint%20Wrapper%20Object%20Reference) (QueryStatus :type EEnvQueryStatus%20Enum :default "Processing"))
  (switch Utilities|FlowControl|Switch|SwitchonEEnvQueryStatus QueryStatus
    (:Success
      (for _array_element (Class|EnvQueryInstanceBlueprintWrapper|GetResultsasLocations QueryInstance)
        (Rendering|Debug|DrawDebugSphere _array_element 5e+01 12 "(R=1.000000,G=0.000000,B=0.442750,A=1.000000)" 2.0 2.0)
        (Game|SpawnActorfromClass "/Game/BluePrint/Charater/BpEnemy.BpEnemy_C" (Math|Transform|MakeTransform _array_element) "AdjustIfPossibleButDontSpawnIfColliding" 0 0)))))

(event EventSpawnNewBot
  (bind _returnvalue (AI|EQS|RunEQSQuery "/Game/BluePrint/Eqs_FindSpawnLocation.Eqs_FindSpawnLocation" self "RandomBest25Pct"))
  (EventDispatchers|AssignOnQueryFinishedEvent _returnvalue (delegate Custom|SpawnQueryFinishedEvent)))

(fn ConstructionScript)