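; Blueprint function library of shortcut getters for the player character, game mode and player controller.
; Each function wraps an engine getter in a cast, using player index 0 for the character and controller, and returns the typed reference.
; The game mode getter returns on both cast outcomes, while the controller getter reaches its return only when the cast succeeds.
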(fn GetBpPlayerCharacter
  (return (.AsBp%20Player%20Character (Utilities|Casting|CastToBpPlayerCharacter (Game|GetPlayerCharacter 0)))))

(fn GetBpGameMode
  (bind _asgame_mode (Utilities|Casting|CastToGameMode (Game|GetGameMode))
    (:then
      _)
    (:CastFailed
      _))
  (return _asgame_mode))

(fn GetBpPlayerController
  (bind _asbp_player_controller_base (Utilities|Casting|CastToBpPlayerControllerBase (Game|GetPlayerController 0)))
  (return _asbp_player_controller_base))